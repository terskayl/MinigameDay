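; BP_BowlingPin is a bowling pin that awards points to the player's BP_ThirdPersonCharacter once when knocked over.
; Tick compares the pin's up vector with world up by dot product and treats a tilt past roughly 45 degrees as knocked.
; Actor overlap records whether the latest overlapping actor was another pin, which earns a higher score.
; The matching Plus3 or Plus6 indicator appears on scoring, and a timer hides it shortly after.
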(event EventBeginPlay
  (Rendering|SetVisibility (Variables|Default|Getplus3) false false)
  (Rendering|SetVisibility (Variables|Default|Getplus6) false false))

(event EventTick
  (params (DeltaSeconds :type Float%20%28single-precision%29))
  (if (< (Math|Vector|DotProduct "0.000000,0.000000,1.000000" (Math|Vector|GetUpVector (Variables|Default|Getpin))) 0.707)
    (Variables|Default|SetKnockedOver true)
    (if (not (Variables|Default|GetContributedScore))
      (bind _asbp_third_person_character (Utilities|Casting|CastToBP_ThirdPersonCharacter (Game|Player|GetPlayerPawn 0)))
      (if (Variables|Default|GetKnockedByOtherPin)
        (Variables|/Game/ThirdPerson/Blueprints/BP_ThirdPersonCharacter.BP_ThirdPersonCharacter_C|SetScore _asbp_third_person_character (+ (Variables|/Game/ThirdPerson/Blueprints/BP_ThirdPersonCharacter.BP_ThirdPersonCharacter_C|GetScore _asbp_third_person_character) 6))
        (Variables|Default|SetContributedScore true)
        (Rendering|SetVisibility (Variables|Default|Getplus6) true false)
        (else
          (Variables|/Game/ThirdPerson/Blueprints/BP_ThirdPersonCharacter.BP_ThirdPersonCharacter_C|SetScore _asbp_third_person_character (+ (Variables|/Game/ThirdPerson/Blueprints/BP_ThirdPersonCharacter.BP_ThirdPersonCharacter_C|GetScore _asbp_third_person_character) 3))
          (Variables|Default|SetContributedScore true)
          (Rendering|SetVisibility (Variables|Default|Getplus3) true false)))
      (Utilities|Time|SetTimerbyFunctionName 0 "hide" 2.0))))

(event Collision|EventActorBeginOverlap
  (params (OtherActor :type Actor%20Object%20Reference))
  (Development|PrintString "knocked")
  (Utilities|Casting|CastToBP_BowlingPin OtherActor
    (:then
      (Development|PrintString "knocked by other pin")
      (Variables|Default|SetKnockedByOtherPin true))
    (:CastFailed
      (Variables|Default|SetKnockedByOtherPin false))))

(fn ConstructionScript)

(fn Hide
  (Rendering|SetVisibility (Variables|Default|Getplus6) false false)
  (Rendering|SetVisibility (Variables|Default|Getplus3) false false))